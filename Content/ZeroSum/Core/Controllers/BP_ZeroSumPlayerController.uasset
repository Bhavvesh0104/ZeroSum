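; BP_ZeroSumPlayerController is the player controller for ZeroSum, handling local player setup when play begins.
; On BeginPlay, only for the local controller, it sets game-only input and hides the mouse cursor.
; It then has the ZeroSum game instance push the username to the server and, if that cast succeeds, creates the player HUD widget and adds it to the viewport.
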(event `self.ReceiveBeginPlay`
  (if (`self.IsLocalPlayerController`)
    (`WidgetBlueprintLibrary.SetInputMode_GameOnly` self)
    (set `self.bShowMouseCursor` false)
    (bind _aszero_sum_game_instance (cast `ZeroSumGameInstance` (`GameplayStatics.GetGameInstance`)))
    (`ZeroSumGameInstance.PushUsernameToServer` _aszero_sum_game_instance self)
    (bind _returnvalue (`|CreateWidget` "/Game/ZeroSum/UI/WBP_PlayerHUD.WBP_PlayerHUD_C" self))
    (`UserWidget.AddToViewport` _returnvalue 0)))

(fn `UserConstructionScript`)