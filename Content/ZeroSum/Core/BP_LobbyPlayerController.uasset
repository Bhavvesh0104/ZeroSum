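; BP_LobbyPlayerController is the player controller for the ZeroSum lobby.
; On BeginPlay, only for the local controller, it creates the lobby widget, adds it to the viewport, switches to UI-only input and shows the mouse cursor.
; It then casts the game instance to ZeroSumGameInstance and calls it to push the player's username to the server.
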(event `self.ReceiveBeginPlay`
  (if (`self.IsLocalPlayerController`)
    (bind _returnvalue (`|CreateWidget` "/Game/ZeroSum/UI/WBP_Lobby.WBP_Lobby_C"))
    (`UserWidget.AddToViewport` _returnvalue 0)
    (`WidgetBlueprintLibrary.SetInputMode_UIOnlyEx` self _returnvalue)
    (set `self.bShowMouseCursor` true)
    (bind _aszero_sum_game_instance (cast `ZeroSumGameInstance` (`GameplayStatics.GetGameInstance`)))
    (`ZeroSumGameInstance.PushUsernameToServer` _aszero_sum_game_instance self)))

(fn `UserConstructionScript`)